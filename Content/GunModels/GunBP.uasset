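; Base-level gun Blueprint that computes the muzzle-to-aim transform for a shot from an assigned player camera.
; CalculateShoot line-traces along the camera's forward vector with debug drawing, then orients a transform at the mesh's Muzzle socket toward the impact point, or the trace end on a miss.
; FireWeapon calls this but does not use the result, so nothing is spawned or damaged, and StopFireWeapon is empty.
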(event `Fire Weapon`
  (`self.CalculateShoot`))

(event `Stop Fire Weapon`)

(fn `CalculateShoot`
  (returns (`ShootTo Location` :type "Transform Structure"))
  (bind _playercamera (`self.PlayerCamera`))
  (bind _returnvalue (`SceneComponent.K2_GetComponentLocation` _playercamera))
  (bind _returnvalue_2 (`SceneComponent.GetSocketLocation` (`self.StaticMesh`) "Muzzle"))
  (bind _returnvalue_3 (+ _returnvalue (* (`SceneComponent.GetForwardVector` _playercamera) 10000000.0)))
  (bind (_outhit _returnvalue_4) (`KismetSystemLibrary.LineTraceSingle` :`Start` _returnvalue :`End` _returnvalue_3 :`TraceChannel` "TraceTypeQuery3" :`DrawDebugType` "ForDuration"))
  (if _returnvalue_4
    (return (`KismetMathLibrary.MakeTransform` _returnvalue_2 (`KismetMathLibrary.FindLookAtRotation` _returnvalue_2 (`.ImpactPoint` (`GameplayStatics.BreakHitResult` _outhit)))))
    (else
      (return (`KismetMathLibrary.MakeTransform` _returnvalue_2 (`KismetMathLibrary.FindLookAtRotation` _returnvalue_2 _returnvalue_3))))))

(fn `Set camera`
  (params (Camera :type "CameraComponent Object Reference"))
  (set `self.PlayerCamera` Camera))

(fn `UserConstructionScript`)